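; Collectible crystal point that flies into the player when the player pawn enters its sphere, then destroys itself.
; On overlap it caches its location, scale and point light intensity, then plays the Crystal_movement timeline.
; Separate timeline tracks lerp it toward the player's current position, shrink it to zero and fade out its light.
; No score is awarded here, and NewFunction_0, a combined version of the three lerps, is never called.
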(event OnComponentBeginOverlap(Sphere)
  (params (OverlappedComponent :type Primitive%20Component%20Object%20Reference) (OtherActor :type Actor%20Object%20Reference) (OtherComp :type Primitive%20Component%20Object%20Reference) (OtherBodyIndex :type Integer) (bFromSweep :type Boolean) (SweepResult :type Hit%20Result%20Structure%20%28by%20ref%29))
  (if (== OtherActor (Game|Player|GetPlayerPawn 0))
    (CallFunction|SetProperties)
    (bind (_direction _lerp_location _lerpscale _crystalintensity) (Timeline|Crystal_movement Play)
      (:Update
        (CallFunction|LOcation _lerp_location)
        (CallFunction|SCale _lerpscale)
        (CallFunction|INtesity _crystalintensity))
      (:Finished
        (Actor|DestroyActor)))))

(event EventBeginPlay)

(event Collision|EventActorBeginOverlap
  (params (OtherActor :type Actor%20Object%20Reference)))

(event EventTick
  (params (DeltaSeconds :type Float%20%28single-precision%29)))

(fn ConstructionScript)

(fn NewFunction0
  (params (A :type Vector) (B :type Vector) (Alpha :type Float%20%28single-precision%29) (Alpha2 :type Float%20%28single-precision%29) (ALpha3 :type Float%20%28single-precision%29))
  (Transformation|SetActorLocation (Math|Vector|Lerp(Vector) A B Alpha) false false)
  (Transformation|SetActorScale3D (Math|Vector|Lerp(Vector) (Variables|CrystalProperties|GetCrystalScale) "0, 0, 0" Alpha2))
  (Rendering|Components|Light|SetIntensity (Variables|Default|GetPointLight) (Math|Float|Lerp (Variables|CrystalProperties|GetCrystalIntensity) 0.0 ALpha3)))

(fn SetProperties
  (Variables|CrystalProperties|SetCrystalLocation (Transformation|GetActorLocation))
  (Variables|CrystalProperties|SetCrystalScale (Transformation|GetActorScale3D))
  (Variables|CrystalProperties|SetCrystalIntensity (Variables|/Script/Engine.LightComponentBase|GetIntensity (Variables|Default|GetPointLight))))

(fn LOcation
  (params (Alpha :type Float%20%28single-precision%29))
  (Transformation|SetActorLocation (Math|Vector|Lerp(Vector) (Variables|CrystalProperties|GetCrystalLocation) (Transformation|GetActorLocation (Game|Player|GetPlayerPawn 0)) Alpha) false false))

(fn SCale
  (params (Alpha :type Float%20%28single-precision%29))
  (Transformation|SetActorScale3D (Math|Vector|Lerp(Vector) (Variables|CrystalProperties|GetCrystalScale) "0, 0, 0" Alpha)))

(fn INtesity
  (params (Alpha :type Float%20%28single-precision%29))
  (Rendering|Components|Light|SetIntensity (Variables|Default|GetPointLight) (Math|Float|Lerp (Variables|CrystalProperties|GetCrystalIntensity) 0.0 Alpha)))